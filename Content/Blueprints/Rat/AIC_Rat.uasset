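; AIC_Rat is the AI controller for a rat that runs to a target point and then vanishes.
; On begin play it spawns a smoke puff at its pawn, waits briefly, then moves to the first TargetPoint actor found in the level.
; When the move succeeds it spawns another puff and destroys the pawn, with no handling for a failed move.
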(event `self.ReceiveBeginPlay`
  (bind _returnvalue (`self.K2_GetPawn`))
  (`NiagaraFunctionLibrary.SpawnSystemAtLocation` "/Game/VFX/NS_SmokePuff.NS_SmokePuff" (`self.K2_GetActorLocation` (`self.K2_GetPawn`)))
  (`KismetSystemLibrary.Delay` 1.0)
  (bind _returnvalue_2 (`GameplayStatics.GetActorOfClass` "/Script/Engine.TargetPoint"))
  (`|AIMoveTo` null (0.0 0.0 0.0) _returnvalue_2
    (:`OnSuccess`
      (`NiagaraFunctionLibrary.SpawnSystemAtLocation` "/Game/VFX/NS_SmokePuff.NS_SmokePuff" (`self.K2_GetActorLocation` _returnvalue))
      (`KismetSystemLibrary.Delay` 0.1)
      (`self.K2_DestroyActor` _returnvalue))))

(fn `UserConstructionScript`)